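; Character preview actor for the inventory screen, showing the player's material, clothing, armor, weapons and backpack on a rotatable mesh.
; A SceneCaptureComponent2D films it, starting inactive and switched by TogglePreview.
; Clothing and armor meshes attach to the main mesh, following its pose via master pose when flagged.
; Weapons and backpack are spawned copies attached to item-defined sockets, with support for primary/secondary swapping and clearing all slots.
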(event `RotateCharacter`
  (params (RotationValue :type "Float (double-precision)"))
  ;[1 1 1] Called from inventory widget
  (`SceneComponent.K2_AddRelativeRotation` (`self.MainMesh`) (`KismetMathLibrary.MakeRotator` 0.0 0.0 RotationValue) false false))

(event `self.ReceiveBeginPlay`
  (bind _returnvalue (`GameplayStatics.GetPlayerCharacter` 0))
  ;[1 1 1] Setting the same material as the player character.
  (`|ExecutionSequence`
    (:`then_0`
      (`/Engine/EditorBlueprintResources/StandardMacros.IsValid` _returnvalue
        (:`Is Valid`
          (`PrimitiveComponent.SetMaterial` (`self.MainMesh`) 0 (`PrimitiveComponent.GetMaterial` (`Character.Mesh` _returnvalue) 0)))))
    (:`then_1`
      (`ActorComponent.Deactivate` (`self.SceneCaptureComponent2D`)))))

(fn `BackpackEquipped`
  (params (BackpackInfo :type "/Game/BattleRoyaleTemplateV2/6-InventoryPickupSystem/System/1-Data/PickupInfos Structure"))
  (bind ((`PickupClass_65_5774673543E64B89847E58BD4193B258` _pickupclass)) (break `/Game/BattleRoyaleTemplateV2/6-InventoryPickupSystem/System/1-Data/PickupInfos` BackpackInfo))
  (`self.IfValidDestroy` (`self.BackpackRef`))
  (if (`KismetSystemLibrary.IsValidClass` _pickupclass)
    (bind _returnvalue (`|SpawnActorFromClass` _pickupclass (`KismetMathLibrary.MakeTransform` (`self.K2_GetActorLocation`)) "AdjustIfPossibleButAlwaysSpawn" "OverrideRootScale" null null))
    (bind _output_get (set `self.BackpackRef` _returnvalue))
    (message `/Game/BattleRoyaleTemplateV2/6-InventoryPickupSystem/System/PickupInterface.UpdateStatus` _output_get "NewEnumerator2")
    (bind _meshref (message `/Game/BattleRoyaleTemplateV2/6-InventoryPickupSystem/System/PickupInterface.GetMeshComponentRef` _output_get))
    (`SceneComponent.K2_AttachToComponent` _meshref (`self.MainMesh`) (`.EquipToSocket_55_A2BBB5EB461E32B8DA49F790C2E6ABBD` (break `/Game/BattleRoyaleTemplateV2/6-InventoryPickupSystem/System/1-Data/PickupInfos` (`local.BackpackInfo`))) "SnapToTarget" "SnapToTarget" "KeepWorld" true)))

(fn `ClearAllSlots`
  (`SkinnedMeshComponent.SetSkinnedAssetAndUpdate` (`self.Skel_HeadArmor`) null true)
  (`SkinnedMeshComponent.SetSkinnedAssetAndUpdate` (`self.Skel_BodyArmor`) null true)
  (`SkinnedMeshComponent.SetSkinnedAssetAndUpdate` (`self.Skel_ClothHead`) null true)
  (`SkinnedMeshComponent.SetSkinnedAssetAndUpdate` (`self.Skel_ClothTopWear`) null true)
  (`SkinnedMeshComponent.SetSkinnedAssetAndUpdate` (`self.Skel_ClothFaceWear`) null true)
  (`SkinnedMeshComponent.SetSkinnedAssetAndUpdate` (`self.Skel_ClothEyeWear`) null true)
  (`SkinnedMeshComponent.SetSkinnedAssetAndUpdate` (`self.Skel_ClothPants`) null true)
  (`SkinnedMeshComponent.SetSkinnedAssetAndUpdate` (`self.Skel_ClothGloves`) null true)
  (`SkinnedMeshComponent.SetSkinnedAssetAndUpdate` (`self.Skel_ClothBoots`) null true)
  (`self.IfValidDestroy` (`self.PrimaryAttached`))
  (`self.IfValidDestroy` (`self.SecondaryAttached`))
  (`self.IfValidDestroy` (`self.PistolAttached`))
  (`self.IfValidDestroy` (`self.MeleeAttached`))
  (`self.IfValidDestroy` (`self.BackpackRef`)))

(fn `IfValidDestroy`
  (params (Target :type "Actor Object Reference"))
  (`/Engine/EditorBlueprintResources/StandardMacros.IsValid` Target
    (:`Is Valid`
      (`self.K2_DestroyActor` Target))))

(fn `PrimaySecondarySwitched`
  (locals (TempRef :type "Actor Object Reference"))
  (bind _secondaryattached (`self.SecondaryAttached`))
  (bind _primaryattached (`self.PrimaryAttached`))
  (`|ExecutionSequence`
    (:`then_0`
      (`/Engine/EditorBlueprintResources/StandardMacros.IsValid` _primaryattached
        (:`Is Valid`
          (bind _info (message `/Game/BattleRoyaleTemplateV2/6-InventoryPickupSystem/System/PickupInterface.GetInfo` _primaryattached))
          (bind _meshref (message `/Game/BattleRoyaleTemplateV2/6-InventoryPickupSystem/System/PickupInterface.GetMeshComponentRef` (`self.PrimaryAttached`)))
          (`SceneComponent.K2_AttachToComponent` _meshref (`self.MainMesh`) (`.UnequipToSocket2_63_AC3A55FD464AC30E79D3F8B725414912` (break `/Game/BattleRoyaleTemplateV2/6-InventoryPickupSystem/System/1-Data/PickupInfos` _info)) "SnapToTarget" "SnapToTarget" "KeepWorld" true))))
    (:`then_1`
      (`/Engine/EditorBlueprintResources/StandardMacros.IsValid` _secondaryattached
        (:`Is Valid`
          (bind _info_2 (message `/Game/BattleRoyaleTemplateV2/6-InventoryPickupSystem/System/PickupInterface.GetInfo` _secondaryattached))
          (bind _meshref_2 (message `/Game/BattleRoyaleTemplateV2/6-InventoryPickupSystem/System/PickupInterface.GetMeshComponentRef` (`self.SecondaryAttached`)))
          (`SceneComponent.K2_AttachToComponent` _meshref_2 (`self.MainMesh`) (`.UnequipToSocket_58_5C84B368499239E9D0BA19AAF73E60DE` (break `/Game/BattleRoyaleTemplateV2/6-InventoryPickupSystem/System/1-Data/PickupInfos` _info_2)) "SnapToTarget" "SnapToTarget" "KeepWorld" true))))
    (:`then_2`
      (set `local.TempRef` (`self.PrimaryAttached`))
      (set `self.PrimaryAttached` (`self.SecondaryAttached`))
      (set `self.SecondaryAttached` (`local.TempRef`)))))

(fn `TogglePreview`
  (params (`Activate?` :type Boolean))
  (bind _scenecapturecomponent2d (`self.SceneCaptureComponent2D`))
  (if `Activate?`
    (`ActorComponent.Activate` _scenecapturecomponent2d false)
    (else
      (`ActorComponent.Deactivate` _scenecapturecomponent2d))))

(fn `UpdateClothBySlot`
  (params (Slot :type "/Game/BattleRoyaleTemplateV2/6-InventoryPickupSystem/System/1-Data/SlotType Enum" :default "NewEnumerator0") (RepClothData :type "/Game/BattleRoyaleTemplateV2/2-BRCharacters/Data/Character_ClothInfo Structure"))
  (locals (TargetMesh :type "SkinnedMeshComponent Object Reference"))
  (bind (_isequipped _skeletatoattach _shouldfollowmeshanimation_ _attachtosocket) (break `/Game/BattleRoyaleTemplateV2/2-BRCharacters/Data/Character_ClothInfo` RepClothData))
  (bind _output_get (set `local.TargetMesh` (select `/Game/BattleRoyaleTemplateV2/6-InventoryPickupSystem/System/1-Data/SlotType` Slot :`NewEnumerator8` (`self.Skel_HeadArmor`) :`NewEnumerator9` (`self.Skel_BodyArmor`) :`NewEnumerator12` (`self.Skel_ClothHead`) :`NewEnumerator13` (`self.Skel_ClothFaceWear`) :`NewEnumerator14` (`self.Skel_ClothEyeWear`) :`NewEnumerator15` (`self.Skel_ClothTopWear`) :`NewEnumerator16` (`self.Skel_ClothPants`) :`NewEnumerator17` (`self.Skel_ClothGloves`) :`NewEnumerator18` (`self.Skel_ClothBoots`) :!type "SkinnedMeshComponent Object Reference")))
  (`SkinnedMeshComponent.SetSkinnedAssetAndUpdate` _output_get (select `bool` _isequipped :`true` _skeletatoattach) true)
  (`SceneComponent.K2_AttachToComponent` (`local.TargetMesh`) (`self.MainMesh`) _attachtosocket "SnapToTarget" "SnapToTarget" "KeepWorld" true)
  (`SkinnedMeshComponent.SetLeaderPoseComponent` (`local.TargetMesh`) (select `bool` (and _isequipped _shouldfollowmeshanimation_) :`true` (`self.MainMesh`) :!type "SkinnedMeshComponent Object Reference") false))

(fn `UserConstructionScript`)

(fn `Weapon Equipped`
  (params (ActorRef :type "Actor Object Reference") (ToSlot :type "/Game/BattleRoyaleTemplateV2/6-InventoryPickupSystem/System/1-Data/SlotType Enum" :default "NewEnumerator0"))
  (bind _secondaryattached (`self.SecondaryAttached`))
  (bind _pistolattached (`self.PistolAttached`))
  (bind _meleeattached (`self.MeleeAttached`))
  (bind _primaryattached (`self.PrimaryAttached`))
  (switch `/Game/BattleRoyaleTemplateV2/6-InventoryPickupSystem/System/1-Data/SlotType` ToSlot
    (:`NewEnumerator2`
      (`/Engine/EditorBlueprintResources/StandardMacros.IsValid` _primaryattached
        (:`Is Valid`
          (`self.K2_DestroyActor` _primaryattached)
          (`/Engine/EditorBlueprintResources/StandardMacros.IsValid` (`local.ActorRef`)
            (:`Is Valid`
              _)))
        (:`Is Not Valid`
          _))
      (bind _returnvalue (`|SpawnActorFromClass` (`GameplayStatics.GetObjectClass` ActorRef) (`KismetMathLibrary.MakeTransform` (`self.K2_GetActorLocation`)) "AdjustIfPossibleButAlwaysSpawn" "OverrideRootScale" null null))
      (bind _output_get (set `self.PrimaryAttached` _returnvalue))
      (message `/Game/BattleRoyaleTemplateV2/6-InventoryPickupSystem/System/PickupInterface.UpdateStatus` _output_get "NewEnumerator2")
      (bind _meshref (message `/Game/BattleRoyaleTemplateV2/6-InventoryPickupSystem/System/PickupInterface.GetMeshComponentRef` _output_get))
      (bind _info (message `/Game/BattleRoyaleTemplateV2/6-InventoryPickupSystem/System/PickupInterface.GetInfo` _output_get))
      (`SceneComponent.K2_AttachToComponent` _meshref (`self.MainMesh`) (`.UnequipToSocket_58_5C84B368499239E9D0BA19AAF73E60DE` (break `/Game/BattleRoyaleTemplateV2/6-InventoryPickupSystem/System/1-Data/PickupInfos` _info)) "SnapToTarget" "SnapToTarget" "KeepWorld" true))
    (:`NewEnumerator3`
      (`/Engine/EditorBlueprintResources/StandardMacros.IsValid` _secondaryattached
        (:`Is Valid`
          (`self.K2_DestroyActor` _secondaryattached)
          (`/Engine/EditorBlueprintResources/StandardMacros.IsValid` (`local.ActorRef`)
            (:`Is Valid`
              _)))
        (:`Is Not Valid`
          _))
      (bind _returnvalue_2 (`|SpawnActorFromClass` (`GameplayStatics.GetObjectClass` (`local.ActorRef`)) (`KismetMathLibrary.MakeTransform` (`self.K2_GetActorLocation`)) "AdjustIfPossibleButAlwaysSpawn" "OverrideRootScale" null null))
      (bind _output_get_2 (set `self.SecondaryAttached` _returnvalue_2))
      (message `/Game/BattleRoyaleTemplateV2/6-InventoryPickupSystem/System/PickupInterface.UpdateStatus` _output_get_2 "NewEnumerator2")
      (bind _meshref_2 (message `/Game/BattleRoyaleTemplateV2/6-InventoryPickupSystem/System/PickupInterface.GetMeshComponentRef` _output_get_2))
      (bind _info_2 (message `/Game/BattleRoyaleTemplateV2/6-InventoryPickupSystem/System/PickupInterface.GetInfo` _output_get_2))
      (`SceneComponent.K2_AttachToComponent` _meshref_2 (`self.MainMesh`) (`.UnequipToSocket2_63_AC3A55FD464AC30E79D3F8B725414912` (break `/Game/BattleRoyaleTemplateV2/6-InventoryPickupSystem/System/1-Data/PickupInfos` _info_2)) "SnapToTarget" "SnapToTarget" "KeepWorld" true))
    (:`NewEnumerator4`
      (`/Engine/EditorBlueprintResources/StandardMacros.IsValid` _pistolattached
        (:`Is Valid`
          (`self.K2_DestroyActor` _pistolattached)
          (`/Engine/EditorBlueprintResources/StandardMacros.IsValid` (`local.ActorRef`)
            (:`Is Valid`
              _)))
        (:`Is Not Valid`
          _))
      (bind _returnvalue_3 (`|SpawnActorFromClass` (`GameplayStatics.GetObjectClass` (`local.ActorRef`)) (`KismetMathLibrary.MakeTransform` (`self.K2_GetActorLocation`)) "AdjustIfPossibleButAlwaysSpawn" "OverrideRootScale" null null))
      (bind _output_get_3 (set `self.PistolAttached` _returnvalue_3))
      (message `/Game/BattleRoyaleTemplateV2/6-InventoryPickupSystem/System/PickupInterface.UpdateStatus` _output_get_3 "NewEnumerator2")
      (bind _meshref_3 (message `/Game/BattleRoyaleTemplateV2/6-InventoryPickupSystem/System/PickupInterface.GetMeshComponentRef` _output_get_3))
      (bind _info_3 (message `/Game/BattleRoyaleTemplateV2/6-InventoryPickupSystem/System/PickupInterface.GetInfo` _output_get_3))
      (`SceneComponent.K2_AttachToComponent` _meshref_3 (`self.MainMesh`) (`.UnequipToSocket_58_5C84B368499239E9D0BA19AAF73E60DE` (break `/Game/BattleRoyaleTemplateV2/6-InventoryPickupSystem/System/1-Data/PickupInfos` _info_3)) "SnapToTarget" "SnapToTarget" "KeepWorld" true))
    (:`NewEnumerator5`
      (`/Engine/EditorBlueprintResources/StandardMacros.IsValid` _meleeattached
        (:`Is Valid`
          (`self.K2_DestroyActor` _meleeattached)
          (`/Engine/EditorBlueprintResources/StandardMacros.IsValid` (`local.ActorRef`)
            (:`Is Valid`
              _)))
        (:`Is Not Valid`
          _))
      (bind _returnvalue_4 (`|SpawnActorFromClass` (`GameplayStatics.GetObjectClass` (`local.ActorRef`)) (`KismetMathLibrary.MakeTransform` (`self.K2_GetActorLocation`)) "AdjustIfPossibleButAlwaysSpawn" "OverrideRootScale" null null))
      (bind _output_get_4 (set `self.MeleeAttached` _returnvalue_4))
      (message `/Game/BattleRoyaleTemplateV2/6-InventoryPickupSystem/System/PickupInterface.UpdateStatus` _output_get_4 "NewEnumerator2")
      (bind _meshref_4 (message `/Game/BattleRoyaleTemplateV2/6-InventoryPickupSystem/System/PickupInterface.GetMeshComponentRef` _output_get_4))
      (bind _info_4 (message `/Game/BattleRoyaleTemplateV2/6-InventoryPickupSystem/System/PickupInterface.GetInfo` _output_get_4))
      (`SceneComponent.K2_AttachToComponent` _meshref_4 (`self.MainMesh`) (`.UnequipToSocket_58_5C84B368499239E9D0BA19AAF73E60DE` (break `/Game/BattleRoyaleTemplateV2/6-InventoryPickupSystem/System/1-Data/PickupInfos` _info_4)) "SnapToTarget" "SnapToTarget" "KeepWorld" true))))